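; BP_BlueDoor is a door that opens for a first-person player holding the blue key.
; A hit on its Cube component casts the other actor to BP_FirstPersonCharacter and checks HaveBlueKey.
; If set, MoveComponentTo animates the door over TumToOpen, targeting a relative Z of OpenHeight plus the actor's world Z and the actor's rotation.
; Debug strings print along the way, and the graph has no closing logic.
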(event `self.Cube.OnComponentHit`
  (params (HitComponent :type "PrimitiveComponent Object Reference") (OtherActor :type "Actor Object Reference") (OtherComp :type "PrimitiveComponent Object Reference") (NormalImpulse :type "Vector Structure") (Hit :type "HitResult Structure (by ref)"))
  (bind _returnvalue (`self.GetTransform`))
  (`KismetSystemLibrary.PrintString` "collision")
  (bind _asbp_first_person_character (cast `/Game/FirstPerson/Blueprints/BP_FirstPersonCharacter` OtherActor))
  (`KismetSystemLibrary.PrintString` "cast first player")
  (if (`/Game/FirstPerson/Blueprints/BP_FirstPersonCharacter.Have Blue Key` _asbp_first_person_character)
    (`KismetSystemLibrary.PrintString` "Opening Door")
    (`KismetSystemLibrary.MoveComponentTo` null (`KismetMathLibrary.MakeVector` 0.0 0.0 (+ (`self.Open Height`) (.z (.location _returnvalue)))) (.rotation _returnvalue) false false (`self.Tum To Open`))))

(fn `UserConstructionScript`
  (`parent.UserConstructionScript`))
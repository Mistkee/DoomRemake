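; Melee enemy with flipbook animations that chases the first-person player, attacks up close and dies when health runs out.
; PawnSensing starts AIMoveTo and latches a sight flag, which Tick uses to face the player and check attack range.
; A DoOnce plays one attack per entry into range, applying damage after the animation and interval delays without rechecking distance.
; AnyDamage reduces health, then plays death and corpse flipbooks before destroying the actor.
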(event `self.ReceiveBeginPlay`
  (bind _output_get (set `self.MaxHealth` (`self.MaxHealth`)))
  (set `self.CurrentHealth` _output_get))

(event `self.ReceiveTick`
  (params (DeltaSeconds :type "Float (single-precision)"))
  (bind _enemyanim (`self.EnemyAnim`))
  (bind (_returnvalue_roll _returnvalue_pitch _returnvalue_yaw) (`KismetMathLibrary.BreakRotator` (`KismetMathLibrary.FindLookAtRotation` (`self.K2_GetActorLocation`) (`self.K2_GetActorLocation` (`GameplayStatics.GetPlayerCharacter` 0)))))
  (if (`self.CanSeePlayer`)
    (`self.K2_SetActorRotation` (`KismetMathLibrary.MakeRotator` 0.0 0.0 _returnvalue_yaw))
    (if (< (`KismetMathLibrary.Vector_Distance` (`self.K2_GetActorLocation` (`GameplayStatics.GetPlayerCharacter` 0)) (`self.K2_GetActorLocation` self)) (`self.AttackDistance`))
      (`/Engine/EditorBlueprintResources/StandardMacros.DoOnce` false :!label _label
        (:`Completed`
          (`ActorComponent.Deactivate` (`self.CharacterMovement`))
          (`PaperFlipbookComponent.SetFlipbook` _enemyanim "/Game/Sprites/Enemy/MeleeEnemy/Attack/EnemyAttack.EnemyAttack")
          (`KismetSystemLibrary.Delay` (`PaperFlipbookComponent.GetFlipbookLength` _enemyanim))
          (`PaperFlipbookComponent.SetFlipbook` (`self.EnemyAnim`) "/Game/Sprites/Enemy/MeleeEnemy/Movement/MeleeIdle.MeleeIdle")
          (`KismetSystemLibrary.Delay` (`self.AttackInterval`))
          (`ActorComponent.Activate` (`self.CharacterMovement`) false)
          (`GameplayStatics.ApplyDamage` (`GameplayStatics.GetPlayerCharacter` 0) (`self.AttackDamage`))))
      (else
        (`PaperFlipbookComponent.SetFlipbook` (`self.EnemyAnim`) "/Game/Sprites/Enemy/MeleeEnemy/Movement/MeleeMove.MeleeMove")
        (goto _label :!via `Reset`)))
    (elif (not (`self.Dead`))
      (`PaperFlipbookComponent.SetFlipbook` (`self.EnemyAnim`) "/Game/Sprites/Enemy/MeleeEnemy/Movement/MeleeIdle.MeleeIdle"))))

(event `self.PawnSensing.OnSeePawn`
  (params (Pawn :type "Pawn Object Reference"))
  (if (`self.Dead`)
    (cast `/Game/FirstPerson/Blueprints/BP_FirstPersonCharacter` Pawn)
    (set `self.CanSeePlayer` false)
    (else
      (bind _asbp_first_person_character (cast `/Game/FirstPerson/Blueprints/BP_FirstPersonCharacter` Pawn))
      (set `self.CanSeePlayer` true)
      (`|AIMoveTo` self (0.0 0.0 0.0) _asbp_first_person_character))))

(event `self.ReceiveAnyDamage`
  (params (Damage :type "Float (single-precision)") (DamageType :type "DamageType Object Reference") (InstigatedBy :type "Controller Object Reference") (DamageCauser :type "Actor Object Reference"))
  (bind _enemyanim (`self.EnemyAnim`))
  (bind _enemyanim_2 (`self.EnemyAnim`))
  (bind _output_get (set `self.CurrentHealth` (- (`self.CurrentHealth`) Damage)))
  (if (<= _output_get 0.0)
    (`/Engine/EditorBlueprintResources/StandardMacros.DoOnce` false
      (:`Completed`
        (`ActorComponent.Deactivate` (`self.CharacterMovement`))
        (set `self.Dead` true)
        (`PaperFlipbookComponent.SetFlipbook` _enemyanim_2 "/Game/Sprites/Enemy/MeleeEnemy/Death/FB_MeleeDeath.FB_MeleeDeath")
        (`KismetSystemLibrary.Delay` (`PaperFlipbookComponent.GetFlipbookLength` _enemyanim_2))
        (`PaperFlipbookComponent.SetFlipbook` _enemyanim "/Game/Sprites/Enemy/MeleeEnemy/Death/FB_DeadBody.FB_DeadBody")
        (`KismetSystemLibrary.Delay` (`PaperFlipbookComponent.GetFlipbookLength` _enemyanim))
        (`self.K2_DestroyActor`)))))

(fn `UserConstructionScript`)
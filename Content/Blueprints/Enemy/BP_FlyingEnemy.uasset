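; Flying enemy with flipbook sprites that searches for the player, fires projectiles on sight and dies from damage.
; Pawn sensing sets a sight flag that stays on while alive; Tick then either yaws toward the player and attacks, or rotates in timed steps to search.
; DoOnce gates reset after delays pace attacks and search turns.
; Lethal damage disables movement, plays the death flipbook and destroys the actor.
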(event `self.PawnSensing.OnSeePawn`
  (params (Pawn :type "Pawn Object Reference"))
  (if (`self.Dead`)
    (cast `/Game/FirstPerson/Blueprints/BP_FirstPersonCharacter` Pawn)
    (set `self.CanSeePlayer` false)
    (else
      (cast `/Game/FirstPerson/Blueprints/BP_FirstPersonCharacter` Pawn)
      (set `self.CanSeePlayer` true))))

(event `self.ReceiveBeginPlay`
  (bind _output_get (set `self.MaxHealth` (`self.MaxHealth`)))
  (set `self.CurrentHealth` _output_get))

(event `Reset Attack`
  (goto _label :!via `Reset`))

(event `self.ReceiveTick`
  (params (DeltaSeconds :type "Float (single-precision)"))
  (bind (_returnvalue_roll _returnvalue_pitch _returnvalue_yaw) (`KismetMathLibrary.BreakRotator` (`KismetMathLibrary.FindLookAtRotation` (`self.K2_GetActorLocation`) (`self.K2_GetActorLocation` (`GameplayStatics.GetPlayerCharacter` 0)))))
  (if (`self.CanSeePlayer`)
    (`self.K2_SetActorRotation` (`KismetMathLibrary.MakeRotator` 0.0 0.0 _returnvalue_yaw))
    (if (not (`self.Dead`))
      (`PaperFlipbookComponent.SetFlipbook` (`self.FlyingEnemyIdle`) "/Game/Sprites/Enemy/BugEnemy/RangedAttack/FlyingEnemyAttack.FlyingEnemyAttack")
      (`/Engine/EditorBlueprintResources/StandardMacros.DoOnce` false :!label _label
        (:`Completed`
          (`self.Attack Player`))))
    (elif (not (`self.Dead`))
      (`/Engine/EditorBlueprintResources/StandardMacros.DoOnce` false :!label _label_2
        (:`Completed`
          (`self.Search For Player`))))))

(event `Reset Search`
  (goto _label_2 :!via `Reset`))

(event `Search For Player`
  (bind (_returnvalue_roll _returnvalue_pitch _returnvalue_yaw) (`KismetMathLibrary.BreakRotator` (`self.K2_GetActorRotation`)))
  (`PaperFlipbookComponent.SetFlipbook` (`self.FlyingEnemyIdle`) "/Game/Sprites/Enemy/BugEnemy/Idle/FlyingEnemyFrame.FlyingEnemyFrame")
  (`KismetSystemLibrary.Delay` (`self.TimeBeforeRotation`))
  (`self.K2_SetActorRotation` (`KismetMathLibrary.MakeRotator` 0.0 0.0 (`self.Rotation`)))
  (if (>= _returnvalue_yaw 360.0)
    (`self.K2_SetActorRotation` (`KismetMathLibrary.MakeRotator` 0.0))
    (else
      (set `self.Rotation` (+ (`self.Rotation`) 90.0))))
  (`self.Reset Search`))

(event `Attack Player`
  (bind (_returnvalue_location _returnvalue_rotation _returnvalue_scale) (`KismetMathLibrary.BreakTransform` (`SceneComponent.K2_GetComponentToWorld` (`self.ProjectileSpawnPos`))))
  (`|SpawnActorFromClass` "/Game/Blueprints/Enemy/BP_EnemyProjectile.BP_EnemyProjectile_C" (`KismetMathLibrary.MakeTransform` _returnvalue_location (`self.K2_GetActorRotation`) _returnvalue_scale) "AlwaysSpawn" "MultiplyWithRoot" null null)
  (`KismetSystemLibrary.Delay` (+ (`PaperFlipbookComponent.GetFlipbookLength` (`self.FlyingEnemyIdle`)) (`self.AtackInterval`)))
  (`self.Reset Attack`))

(event `self.ReceiveAnyDamage`
  (params (Damage :type "Float (single-precision)") (DamageType :type "DamageType Object Reference") (InstigatedBy :type "Controller Object Reference") (DamageCauser :type "Actor Object Reference"))
  (bind _flyingenemyidle (`self.FlyingEnemyIdle`))
  (bind _output_get (set `self.CurrentHealth` (- (`self.CurrentHealth`) Damage)))
  (if (<= _output_get 0.0)
    (`ActorComponent.Deactivate` (`self.CharacterMovement`))
    (`/Engine/EditorBlueprintResources/StandardMacros.DoOnce` false
      (:`Completed`
        (`ActorComponent.K2_DestroyComponent` (`self.FlyingEnemyIdle1`))
        (set `self.Dead` true)
        (`PaperFlipbookComponent.SetFlipbook` _flyingenemyidle "/Game/Sprites/Enemy/BugEnemy/Death/FlyingEnemyDeath.FlyingEnemyDeath")
        (`KismetSystemLibrary.Delay` (`PaperFlipbookComponent.GetFlipbookLength` _flyingenemyidle))
        (`self.K2_DestroyActor`)))))

(fn `UserConstructionScript`)
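; BP_HealthItem is a health pickup that works on BP_FirstPersonCharacter when it overlaps the item's Sphere component.
; It acts only if the character's CurrentHealth equals exactly 100, adding HealthContent to that value.
; It then calls the character's CheckForOverhealth and destroys itself; at any other health value the item stays in place.
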(event `self.Sphere.OnComponentBeginOverlap`
  (params (OverlappedComponent :type "PrimitiveComponent Object Reference") (OtherActor :type "Actor Object Reference") (OtherComp :type "PrimitiveComponent Object Reference") (OtherBodyIndex :type Integer) (bFromSweep :type Boolean) (SweepResult :type "HitResult Structure (by ref)"))
  (bind _asbp_first_person_character (cast `/Game/FirstPerson/Blueprints/BP_FirstPersonCharacter` OtherActor))
  (bind _current_health (`/Game/FirstPerson/Blueprints/BP_FirstPersonCharacter.Current Health` _asbp_first_person_character))
  (if (== _current_health 100.0)
    (set `/Game/FirstPerson/Blueprints/BP_FirstPersonCharacter.Current Health` (+ _current_health (`self.Health Content`)) _asbp_first_person_character)
    (`/Game/FirstPerson/Blueprints/BP_FirstPersonCharacter.Check For Overhealth` _asbp_first_person_character)
    (`self.K2_DestroyActor`)))

(fn `UserConstructionScript`
  (`parent.UserConstructionScript`))
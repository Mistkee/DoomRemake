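; BP_Pistol is a pistol weapon that fires using its own ammo count and flipbook animation.
; ShootWeapon checks for ammo, then a DoOnce gate calls FireWeapon, plays the fire flipbook and spends one round.
; After a delay matching the flipbook length, it returns to idle, resets the gate and refreshes the HUD.
; AddAmmo adds received ammo to the count, clears the received amount and updates the HUD.
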(event `self.ReceiveBeginPlay`
  (`parent.ReceiveBeginPlay`))

(event `Add Ammo`
  (set `self.PistolAmmo` (+ (`self.PistolAmmo`) (`self.ReceivedAmmo`)))
  (set `self.ReceivedAmmo` 0)
  (bind _asnew_hud (cast `/Game/Blueprints/HUD/NewHUD` (`PlayerController.GetHUD` (`GameplayStatics.GetPlayerController` 0))))
  (`/Game/Blueprints/HUD/WB_PlayerHUD.UpdateAmmo` (`/Game/Blueprints/HUD/NewHUD.UI Ref` _asnew_hud)))

(event `self.ShootWeapon`
  (bind _weaponflipbook (`self.WeaponFlipbook`))
  (if (> (`self.PistolAmmo`) 0)
    (`/Engine/EditorBlueprintResources/StandardMacros.DoOnce` false :!label _label
      (:`Completed`
        (`self.FireWeapon`)
        (`PaperFlipbookComponent.SetFlipbook` _weaponflipbook "/Game/Sprites/Weapons/Pistol/pistolFire.pistolFire")
        (set `self.PistolAmmo` (- (`self.PistolAmmo`) 1))
        (`KismetSystemLibrary.Delay` (`PaperFlipbookComponent.GetFlipbookLength` _weaponflipbook))
        (`PaperFlipbookComponent.SetFlipbook` (`self.WeaponFlipbook`) "/Game/Sprites/Weapons/Pistol/pistolIdle.pistolIdle")
        (`self.ResetWeapon`)
        (bind _asnew_hud (cast `/Game/Blueprints/HUD/NewHUD` (`PlayerController.GetHUD` (`GameplayStatics.GetPlayerController` 0))))
        (`/Game/Blueprints/HUD/WB_PlayerHUD.UpdateAmmo` (`/Game/Blueprints/HUD/NewHUD.UI Ref` _asnew_hud))))))

(event `ResetWeapon`
  (goto _label :!via `Reset`))

(fn `UserConstructionScript`
  (`parent.UserConstructionScript`))
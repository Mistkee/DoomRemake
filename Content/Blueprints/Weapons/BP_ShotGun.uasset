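; Shotgun weapon Blueprint that fires while the player character has shotgun ammo, using flipbook sprites for its animation.
; ShootWeapon reads ShotgunAmmo from BP_FirstPersonCharacter and passes a DoOnce gate, then calls FireWeapon, plays the fire flipbook and decrements the ammo.
; After a delay equal to the flipbook's length, it restores the idle flipbook and calls ResetWeapon to reopen the gate, limiting fire rate to the animation.
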(event `self.ShootWeapon`
  (bind _weaponflipbook (`self.WeaponFlipbook`))
  (bind _asbp_first_person_character (cast `/Game/FirstPerson/Blueprints/BP_FirstPersonCharacter` (`GameplayStatics.GetPlayerCharacter` 0)))
  (bind _shotgun_ammo (`/Game/FirstPerson/Blueprints/BP_FirstPersonCharacter.Shotgun Ammo` _asbp_first_person_character))
  (if (> _shotgun_ammo 0)
    (`/Engine/EditorBlueprintResources/StandardMacros.DoOnce` false :!label _label
      (:`Completed`
        (`self.FireWeapon`)
        (`PaperFlipbookComponent.SetFlipbook` _weaponflipbook "/Game/Sprites/Weapons/Shotgun/ShotgunFire.ShotgunFire")
        (set `/Game/FirstPerson/Blueprints/BP_FirstPersonCharacter.Shotgun Ammo` (- _shotgun_ammo 1) _asbp_first_person_character)
        (`KismetSystemLibrary.Delay` (`PaperFlipbookComponent.GetFlipbookLength` _weaponflipbook))
        (`PaperFlipbookComponent.SetFlipbook` (`self.WeaponFlipbook`) "/Game/Sprites/Weapons/Shotgun/ShotgunIdle.ShotgunIdle")
        (`self.ResetWeapon`)))))

(event `ResetWeapon`
  (goto _label :!via `Reset`))

(fn `UserConstructionScript`
  (`parent.UserConstructionScript`))
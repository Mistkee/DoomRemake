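; BP_BaseWeapon is a base weapon Blueprint that provides hitscan firing.
; FireWeapon line-traces forward from the LineTrace component over LineTraceDistance against static, dynamic and pawn objects, then applies WeaponDamage to any hit actor.
; The trace leaves debug drawing on for a duration.
; ShootWeapon and StopShooting are empty events, and nothing in this graph calls FireWeapon.
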(event `ShootWeapon`)

(event `StopShooting`)

(fn `FireWeapon`
  (bind _returnvalue (`SceneComponent.K2_GetComponentLocation` (`self.LineTrace`)))
  (bind (_outhit _returnvalue_2) (`KismetSystemLibrary.LineTraceSingleForObjects` :`Start` _returnvalue :`End` (+ _returnvalue (* (`KismetMathLibrary.GetForwardVector` (`SceneComponent.K2_GetComponentRotation` (`self.LineTrace`))) (`self.LineTraceDistance`))) :`ObjectTypes` (`|MakeArray` "ObjectTypeQuery1" "ObjectTypeQuery2" "ObjectTypeQuery3" :!type "EObjectTypeQuery Enum") :`DrawDebugType` "ForDuration"))
  (if _returnvalue_2
    (`GameplayStatics.ApplyDamage` (`.HitActor` (`GameplayStatics.BreakHitResult` _outhit)) (`self.WeaponDamage`))))

(fn `UserConstructionScript`)